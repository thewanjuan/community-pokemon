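; Blueprint function library for the fluid interaction tool that stamps fluid disturbances into a fluid controller's render targets.
; DrawFluidSim sets location, size and intensity on a draw material and renders it to the current height target; the Capture variant omits size and intensity and uses GetRT.
; Both compute world-grid cell bounds from location and the MPC ViewDistance for UV offsetting.
; DistanceCheck returns point separation and an out-of-radius flag.
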(fn DrawFluidSim
  (params (Fluid%20Controller :type BP%20Fluid%20Controller%20Object%20Reference%20%28by%20ref%29) (Draw%20Material :type Material%20Instance%20Dynamic%20Object%20Reference%20%28by%20ref%29) (Draw%20Location :type Vector) (Draw%20Size :type Float%20%28single-precision%29) (Draw%20Intensity :type Float%20%28single-precision%29))
  ;[1 1 1] Draw Fluid Spot
  (Utilities|IsValid Fluid%20Controller ; Check if fluid controller is valid
    (:Is%20Valid
      (Utilities|IsValid Draw%20Material ; Check if Draw Material is Valid
        (:Is%20Valid
          (bind _rendertarget (Default|GetRTHeight Fluid%20Controller (Variables|/Game/FluidInteractionTool/Blueprints/BP_FluidController.BP_FluidController_C|GetCurrentRT Fluid%20Controller)))
          (bind _returnvalue (Rendering|Material|GetScalarParameterValue Fluid%20Controller "/Game/FluidInteractionTool/Blueprints/Data/MPC_FluidInteraction.MPC_FluidInteraction" "ViewDistance" :!class /Script/Engine.KismetMaterialLibrary)) ; Get the Global View Distance Param
          ;;[1 1 1] Set the fluid draw parameters
          (Rendering|Material|SetScalarParameterValue Draw%20Material "RenderTargetSize" (Math|Conversions|ToFloat(Integer) (Variables|/Game/FluidInteractionTool/Blueprints/BP_FluidController.BP_FluidController_C|GetRenderTargetSize Fluid%20Controller)) :!class /Script/Engine.MaterialInstanceDynamic)
          (Rendering|Material|SetVectorParameterValue Draw%20Material "XXYY" (Utilities|Struct|MakeLinearColor (select (< (.X (Math|Vector|BreakVector (/ Draw%20Location _returnvalue))) 0.0) (Math|Conversions|ToFloat(Integer) (- (Math|Float|Truncate (.X (Math|Vector|BreakVector (/ Draw%20Location _returnvalue)))) 1)) (Math|Conversions|ToFloat(Integer) (Math|Float|Truncate (.X (Math|Vector|BreakVector (/ Draw%20Location _returnvalue)))))) (select (< (.X (Math|Vector|BreakVector (/ Draw%20Location _returnvalue))) 0.0) (Math|Conversions|ToFloat(Integer) (Math|Float|Truncate (.X (Math|Vector|BreakVector (/ Draw%20Location _returnvalue))))) (Math|Conversions|ToFloat(Integer) (+ (Math|Float|Truncate (.X (Math|Vector|BreakVector (/ Draw%20Location _returnvalue)))) 1))) (select (< (.Y (Math|Vector|BreakVector (/ Draw%20Location _returnvalue))) 0.0) (Math|Conversions|ToFloat(Integer) (- (Math|Float|Truncate (.Y (Math|Vector|BreakVector (/ Draw%20Location _returnvalue)))) 1)) (Math|Conversions|ToFloat(Integer) (Math|Float|Truncate (.Y (Math|Vector|BreakVector (/ Draw%20Location _returnvalue)))))) (select (< (.Y (Math|Vector|BreakVector (/ Draw%20Location _returnvalue))) 0.0) (Math|Conversions|ToFloat(Integer) (Math|Float|Truncate (.Y (Math|Vector|BreakVector (/ Draw%20Location _returnvalue))))) (Math|Conversions|ToFloat(Integer) (+ (Math|Float|Truncate (.Y (Math|Vector|BreakVector (/ Draw%20Location _returnvalue)))) 1)))) :!class /Script/Engine.MaterialInstanceDynamic)
          (Rendering|Material|SetVectorParameterValue Draw%20Material "Location" (Math|Conversions|ToLinearColor(Vector) Draw%20Location) :!class /Script/Engine.MaterialInstanceDynamic)
          (Rendering|Material|SetScalarParameterValue Draw%20Material "DrawSize" Draw%20Size :!class /Script/Engine.MaterialInstanceDynamic)
          (Rendering|Material|SetScalarParameterValue Draw%20Material "DrawIntensity" Draw%20Intensity :!class /Script/Engine.MaterialInstanceDynamic)
          (Rendering|DrawMaterialtoRenderTarget Fluid%20Controller _rendertarget Draw%20Material) ; Draw Fluid to render target
        )))))

(fn DistanceCheck
  (params (Location%201 :type Vector) (Location%202 :type Vector) (Distance%20Radius :type Float%20%28single-precision%29))
  (bind _returnvalue (- Location%201 Location%202))
  (bind _returnvalue_2 (Math|Vector|VectorLength _returnvalue))
  (bind _returnvalue_3 (Math|Float|Absolute(Float) _returnvalue_2))
  ;[1 1 1] Simple Distance Check
  (return _returnvalue_3 (> (/ _returnvalue_3 Distance%20Radius) 1.0)))

(fn DrawFluidSimCapture
  (params (Fluid%20Controller :type BP%20Fluid%20Controller%20Object%20Reference%20%28by%20ref%29) (Draw%20Material :type Material%20Instance%20Dynamic%20Object%20Reference%20%28by%20ref%29) (Draw%20Location :type Vector))
  ;[1 1 1] Draw Fluid Spot
  (Utilities|IsValid Fluid%20Controller ; Check if fluid controller is valid
    (:Is%20Valid
      (Utilities|IsValid Draw%20Material ; Check if Draw Material is Valid
        (:Is%20Valid
          (bind _rendertarget (Default|GetRT Fluid%20Controller (Variables|/Game/FluidInteractionTool/Blueprints/BP_FluidController.BP_FluidController_C|GetCurrentRT Fluid%20Controller))) ; Get Current Height RT
          (bind _returnvalue (Rendering|Material|GetScalarParameterValue Fluid%20Controller "/Game/FluidInteractionTool/Blueprints/Data/MPC_FluidInteraction.MPC_FluidInteraction" "ViewDistance" :!class /Script/Engine.KismetMaterialLibrary)) ; Get the Global View Distance Param
          ;;[1 1 1] Set the fluid draw parameters
          (Rendering|Material|SetScalarParameterValue Draw%20Material "RenderTargetSize" (Math|Conversions|ToFloat(Integer) (Variables|/Game/FluidInteractionTool/Blueprints/BP_FluidController.BP_FluidController_C|GetRenderTargetSize Fluid%20Controller)) :!class /Script/Engine.MaterialInstanceDynamic)
          (Rendering|Material|SetVectorParameterValue Draw%20Material "XXYY" (Utilities|Struct|MakeLinearColor (select (< (.X (Math|Vector|BreakVector (/ Draw%20Location _returnvalue))) 0.0) (Math|Conversions|ToFloat(Integer) (- (Math|Float|Truncate (.X (Math|Vector|BreakVector (/ Draw%20Location _returnvalue)))) 1)) (Math|Conversions|ToFloat(Integer) (Math|Float|Truncate (.X (Math|Vector|BreakVector (/ Draw%20Location _returnvalue)))))) (select (< (.X (Math|Vector|BreakVector (/ Draw%20Location _returnvalue))) 0.0) (Math|Conversions|ToFloat(Integer) (Math|Float|Truncate (.X (Math|Vector|BreakVector (/ Draw%20Location _returnvalue))))) (Math|Conversions|ToFloat(Integer) (+ (Math|Float|Truncate (.X (Math|Vector|BreakVector (/ Draw%20Location _returnvalue)))) 1))) (select (< (.Y (Math|Vector|BreakVector (/ Draw%20Location _returnvalue))) 0.0) (Math|Conversions|ToFloat(Integer) (- (Math|Float|Truncate (.Y (Math|Vector|BreakVector (/ Draw%20Location _returnvalue)))) 1)) (Math|Conversions|ToFloat(Integer) (Math|Float|Truncate (.Y (Math|Vector|BreakVector (/ Draw%20Location _returnvalue)))))) (select (< (.Y (Math|Vector|BreakVector (/ Draw%20Location _returnvalue))) 0.0) (Math|Conversions|ToFloat(Integer) (Math|Float|Truncate (.Y (Math|Vector|BreakVector (/ Draw%20Location _returnvalue))))) (Math|Conversions|ToFloat(Integer) (+ (Math|Float|Truncate (.Y (Math|Vector|BreakVector (/ Draw%20Location _returnvalue)))) 1)))) :!class /Script/Engine.MaterialInstanceDynamic)
          (Rendering|Material|SetVectorParameterValue Draw%20Material "Location" (Math|Conversions|ToLinearColor(Vector) Draw%20Location) :!class /Script/Engine.MaterialInstanceDynamic)
          (Rendering|DrawMaterialtoRenderTarget Fluid%20Controller _rendertarget Draw%20Material) ; Draw Fluid to render target
        )))))