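; Demo rain actor that makes raindrop impacts disturb a fluid simulation.
; On BeginPlay it creates a dynamic instance of the fluid draw material.
; Each PS_Rain particle collision within a set radius of the player camera calls DrawFluidSim on the referenced fluid controller at the hit location, using randomized small size and intensity.
; Collisions beyond that camera distance are skipped.
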(event OnParticleCollide(PS_Rain)
  (params (EventName :type Name :default "None") (EmitterTime :type Float%20%28single-precision%29) (ParticleTime :type Integer) (Location :type Vector) (Velocity :type Vector :default "0, 0, 0") (Direction :type Vector :default "0, 0, 0") (Normal :type Vector :default "0, 0, 0") (BoneName :type Name :default "None") (PhysMat :type Physical%20Material%20Object%20Reference))
  (bind _returnvalue (Game|GetPlayerCameraManager 0))
  (Utilities|IsValid (Variables|Default|GetFluidDrawMaterialInstanceDynamic)
    (:Is%20Valid
      (Utilities|IsValid (Variables|Default|GetFluidControllerReference)
        (:Is%20Valid
          (Utilities|IsValid _returnvalue
            (:Is%20Valid
              (bind _outofradius (CallFunction|DistanceCheck (Camera|GetCameraLocation _returnvalue) Location 4e+03))
              (if (not _outofradius)
                (CallFunction|DrawFluidSim (Variables|Default|GetFluidControllerReference) (Variables|Default|GetFluidDrawMaterialInstanceDynamic) Location (Math|Random|RandomFloatinRange 0.0005 0.001) (Math|Random|RandomFloatinRange 0.1 0.2))))))))))

(event EventBeginPlay
  ;[1 0.5 0] Create Fluid Draw Material Instance Dynamic for the Draw Fluid Sim
  (bind _returnvalue (Rendering|Material|CreateDynamicMaterialInstance "/Game/FluidInteractionTool/Blueprints/Data/M_FluidDraw.M_FluidDraw" :!class /Script/Engine.KismetMaterialLibrary))
  (Variables|Default|SetFluidDrawMaterialInstanceDynamic _returnvalue))

(fn ConstructionScript)