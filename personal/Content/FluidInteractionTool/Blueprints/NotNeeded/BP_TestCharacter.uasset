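; BP_TestCharacter is a simple test character that walks, looks around, jumps and fires bullets.
; Left click spawns a BP_Bullet above the actor, gives it a limited lifetime and launches its mesh along the control rotation with a velocity-change impulse.
; Raw key events handle jumping and toggle a forward-movement flag that Tick turns into movement input, while mouse axes drive yaw and inverted pitch.
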(event EventBeginPlay)

(event EventTick
  (params (DeltaSeconds :type Float%20%28single-precision%29))
  (Utilities|FlowControl|Sequence
    (:then_0
      (if (Variables|Default|GetMoveForward)
        (Pawn|Input|AddMovementInput (Transformation|GetActorForwardVector) 1.0 false)))))

(event Input|MouseEvents|MouseX
  (params (AxisValue :type Float%20%28single-precision%29))
  (Pawn|Input|AddControllerYawInput AxisValue))

(event Input|MouseEvents|MouseY
  (params (AxisValue :type Float%20%28single-precision%29))
  (Pawn|Input|AddControllerPitchInput (* AxisValue -1.0)))

(event Input|KeyboardEvents|W
  (params (Key :type Key%20Structure :default "AnyKey"))
  (:Pressed
    (Variables|Default|SetMoveForward true))
  (:Released
    (Variables|Default|SetMoveForward false)))

(event Input|KeyboardEvents|SpaceBar
  (params (Key :type Key%20Structure :default "AnyKey"))
  (:Pressed
    (Character|Jump)))

(event Input|MouseEvents|LeftMouseButton
  (params (Key :type Key%20Structure :default "AnyKey"))
  (:Pressed
    (bind _returnvalue (Game|SpawnActorfromClass "/Game/FluidInteractionTool/Blueprints/NotNeeded/BP_Bullet.BP_Bullet_C" (Math|Transform|MakeTransform (+ (Transformation|GetActorLocation) "0.000000, 0,150.000000") "0, 0, 0" "1.000000,1.000000,1.000000") "AlwaysSpawn" 0 0))
    (Actor|SetLifeSpan _returnvalue 1e+01)
    (Physics|AddImpulse (Variables|/Game/FluidInteractionTool/Blueprints/NotNeeded/BP_Bullet.BP_Bullet_C|GetStaticMesh _returnvalue) (* (Math|Vector|GetForwardVector (Pawn|GetControlRotation :!class /Script/Engine.Pawn)) 1.5e+03) "None" true)))

(fn ConstructionScript)